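; Base enemy that chases the player character, makes melee attacks and ragdolls when its health runs out.
; Tick reissues AIMoveTo every frame, even after death, and while alive sphere-traces forward from an arrow component to detect the first-person character.
; Detection starts an attack montage that repeats while in range; its "Damage" notify applies full radial damage around the enemy.
; AnyDamage lowers health and sets the dead flag.
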(event Custom|Attack
  (if (Variables|Default|GetEnemyInRange?)
    (if (not (Class|AnimInstance|IsAnyMontagePlaying (Components|SkeletalMesh|GetAnimInstance (Variables|Character|GetMesh))))
      (bind _notifyname (Animation|Montage|PlayMontage (Variables|Character|GetMesh) (Variables|Default|GetAnim%20Montage))
        (:OnCompleted
          (if (Variables|Default|GetEnemyInRange?)
            (CallFunction|Attack)))
        (:OnNotifyBegin
          (if (== _notifyname "Damage")
            (CallFunction|DamagePlayer)))))))

(event Custom|Damage%20Player
  (Game|Damage|ApplyRadialDamage 25.0 (Transformation|GetActorLocation) 1.5e+02 0 (Utilities|Array|MakeArray self) self 0 true "ECC_Visibility"))

(event Game|Damage|EventAnyDamage
  (params (Damage :type Float%20%28single-precision%29) (DamageType :type Damage%20Type%20Object%20Reference) (InstigatedBy :type Controller%20Object%20Reference) (DamageCauser :type Actor%20Object%20Reference))
  (bind _output_get (Variables|Default|SetCurrentHealth (- (Variables|Default|GetCurrentHealth) Damage)))
  (if (<= (Math|Float|Clamp(Float) _output_get 0.0 (Variables|Default|GetMaxHealth)) 0.0)
    (Physics|SetSimulatePhysics (Variables|Character|GetMesh) true)
    (Variables|Default|SetDead true)
    (else
      (Variables|Default|SetDead false))))

(event EventTick
  (params (DeltaSeconds :type Float%20%28single-precision%29))
  (bind _arrow1 (Variables|Default|GetArrow1))
  (bind _returnvalue (Transformation|GetWorldLocation _arrow1))
  (Utilities|FlowControl|Sequence
    (:then_0
      (AI|AIMoveTo self "0, 0, 0" (Game|GetPlayerCharacter 0) 5e+01 false))
    (:then_1
      (if (not (Variables|Default|GetDead))
        (bind (_outhit _returnvalue_2) (Collision|SphereTraceByChannel _returnvalue (+ _returnvalue (* (Math|Vector|GetForwardVector _arrow1) 1e+02)) 8.0 "TraceTypeQuery1" false (Utilities|Array|MakeArray self) "None"))
        (if (and _returnvalue_2 (.bSuccess (Utilities|Casting|CastToBP_FirstPersonCharacter (.HitActor (Collision|BreakHitResult _outhit)))))
          (Variables|Default|SetEnemyInRange? true)
          (CallFunction|Attack)
          (else
            (Variables|Default|SetEnemyInRange? false)))))))

(fn ConstructionScript)